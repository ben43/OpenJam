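; BP_Breakable is a movable actor that shatters into a destructible mesh and damages its surroundings.
; Its childFunction override calls the parent, then replaces the static mesh with a runtime-added, scaled-up destructible component at the same world location, using DestroyedMesh.
; The new component simulates physics and takes immediate damage to fracture it, followed by heavy radial damage around that point.
; The event graph is unused, so the parent decides when this runs.
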(fn `childFunction`
  (locals (forwardVector :type "Vector Structure") (WorldLocation :type "Vector Structure"))
  (bind _worldlocation (`local.WorldLocation`))
  (`parent.childFunction`)
  (set `local.WorldLocation` (`SceneComponent.K2_GetComponentLocation` (`self.StaticMesh`)))
  (`ActorComponent.K2_DestroyComponent` (`self.StaticMesh`))
  (bind _returnvalue (`|AddComponentByClass` "/Script/ApexDestruction.DestructibleComponent" false (`KismetMathLibrary.MakeTransform` (0.0 0.0 0.0) (struct) (5.0 5.0 5.0))))
  (`DestructibleComponent.SetDestructibleMesh` _returnvalue (`self.destroyedMesh`))
  (`SceneComponent.K2_SetWorldLocation` _returnvalue (`local.WorldLocation`) false true)
  (`PrimitiveComponent.SetSimulatePhysics` _returnvalue true)
  (`DestructibleComponent.ApplyDamage` _returnvalue 1000.0 _worldlocation _worldlocation 100.0)
  (`GameplayStatics.ApplyRadialDamage` :`BaseDamage` 100000.0 :`Origin` _worldlocation :`DamageRadius` 1000.0 :`DamageTypeClass` "/Script/Engine.DamageType" :`DamageCauser` null :`InstigatedByController` null))

(fn `UserConstructionScript`
  (`parent.UserConstructionScript`))
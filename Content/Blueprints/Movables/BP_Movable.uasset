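; Base wreckable prop Blueprint that awards score when knocked hard enough after contact with the chaser.
; Chaser overlap with the box enables mesh physics, removes the box and starts a looping timer that checks velocity against a threshold.
; Crossing it stops the timer once, calls an empty ChildFunction hook, adds WreckScore to the game state and briefly shows a score widget.
; The construction script applies the configurable Model mesh.
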(event `self.ReceiveBeginPlay`
  ;[1 1 1] Get Reference to the chaser
  (bind _returnvalue (`/Game/Blueprints/FunctionLibrary.GetChaserReference`))
  (set `self.ChaserReference` _returnvalue))

(event `self.Box.OnComponentBeginOverlap`
  (params (OverlappedComponent :type "PrimitiveComponent Object Reference") (OtherActor :type "Actor Object Reference") (OtherComp :type "PrimitiveComponent Object Reference") (OtherBodyIndex :type Integer) (bFromSweep :type Boolean) (SweepResult :type "HitResult Structure (by ref)"))
  (if (== OtherActor (`self.ChaserReference`))
    ;[1 1 1] Set simulate physics, destroy HitBox and start the Timer for velocity check.
    (`PrimitiveComponent.SetSimulatePhysics` (`self.StaticMesh`) true)
    (`ActorComponent.K2_DestroyComponent` (`self.Box`))
    (`self.StartTimer`)))

(event `StartTimer`
  ;[1 1 1] Checks velocity to see if it is wrecked
  (bind _returnvalue (`KismetSystemLibrary.K2_SetTimerDelegate` (delegate `CheckVelocity`) 0.1 true)))

(event `CheckVelocity`
  ;[1 1 1] Checks velocity to see if it is wrecked
  (if (`self.Velocity` (`self.Velocity Threshold`))
    (`/Engine/EditorBlueprintResources/StandardMacros.DoOnce` false
      (:`Completed`
        (`KismetSystemLibrary.K2_ClearAndInvalidateTimerHandle` (stale `StartTimer` _returnvalue))
        (`self.childFunction`)
        (`self.AddScore`)
        (`self.SpawnWidgetScore`)))))

(event `SpawnWidgetScore`
  ;[1 1 1] Spawn Widget Score
  (bind _aswgt_wreckable_inagame_score (cast `/Game/UI/UiElements/WGT_Wreckable_InagameScore` (`WidgetComponent.GetUserWidgetObject` (`self.Widget`))))
  (set `/Game/UI/UiElements/WGT_Wreckable_InagameScore.Score` (`KismetStringLibrary.Conv_IntToString` (`self.WreckScore`)) _aswgt_wreckable_inagame_score)
  (`/Game/UI/UiElements/WGT_Wreckable_InagameScore.SpawnScore` _aswgt_wreckable_inagame_score)
  (`KismetSystemLibrary.Delay` 1.0)
  (`ActorComponent.K2_DestroyComponent` (`self.Widget`)))

(event `AddScore`
  ;[1 1 1] Update Score in Player Hud
  (bind _asmy_game_state (cast `/Game/Blueprints/myGameState` (`GameplayStatics.GetGameState`)))
  (set `/Game/Blueprints/myGameState.Score` (+ (`/Game/Blueprints/myGameState.Score` _asmy_game_state) (`self.WreckScore`)) _asmy_game_state))

(fn `childFunction`)

(fn `UserConstructionScript`
  (`StaticMeshComponent.SetStaticMesh` (`self.StaticMesh`) (`self.Model`))
  (set `self.WreckScore` (`self.WreckScore`)))

(fn `Velocity`
  (params (VelocityThreshold :type "Float (double-precision)"))
  (returns (ReturnValue :type Boolean))
  (return (>= (`KismetMathLibrary.VSize` (`SceneComponent.GetComponentVelocity` (`self.StaticMesh`))) VelocityThreshold)))
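; BP_SaveScore holds an array of integer scores and provides a sortScore event that orders them from highest to lowest.
; The event runs a selection sort, repeatedly moving the maximum value found by MaxOfIntArray from Scores into TempScore.
; It then copies the sorted result back into Scores and clears the temporary array.
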(event `sortScore`
  (bind _tempscore (`self.tempScore`))
  (bind (_indexofmaxvalue _maxvalue) (`KismetMathLibrary.MaxOfIntArray` (`self.Scores`)))
  (bind _output_get (set `self.ScoreLength` (- (`KismetArrayLibrary.Array_Length` (`self.Scores`)) 1)))
  (for _ (range (+ _output_get 1))
    (`KismetArrayLibrary.Array_Add` (`self.tempScore`) _maxvalue)
    (`KismetArrayLibrary.Array_Remove` (`self.Scores`) _indexofmaxvalue))
  (set `self.Scores` _tempscore)
  (`KismetArrayLibrary.Array_Clear` _tempscore))
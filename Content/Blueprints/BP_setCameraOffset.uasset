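; Trigger volume that blends the player's camera to its own configured framing when the player character overlaps its box.
; On overlap it snapshots the spring arm's offsets, length and camera rotation, then starts a looping timer.
; Each tick lerps them toward the target values by an incrementing alpha, clearing the timer only when alpha exactly equals one.
; Construction script and Set Spring Arm apply the spring arm targets directly.
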(event `self.ReceiveBeginPlay`
  (bind _asbp_player (cast `/Game/Blueprints/Players/BP_Player` (`GameplayStatics.GetPlayerCharacter` 0)))
  (set `self.characterRef` _asbp_player))

(event `self.Box.OnComponentBeginOverlap`
  (params (OverlappedComponent :type "PrimitiveComponent Object Reference") (OtherActor :type "Actor Object Reference") (OtherComp :type "PrimitiveComponent Object Reference") (OtherBodyIndex :type Integer) (bFromSweep :type Boolean) (SweepResult :type "HitResult Structure (by ref)"))
  (bind _returnvalue (`GameplayStatics.GetPlayerCharacter` 0))
  (if (== OtherActor _returnvalue)
    (bind _asbp_player (cast `/Game/Blueprints/Players/BP_Player` _returnvalue))
    (bind _springarm (`/Game/Blueprints/Players/BP_Player.SpringArm` _asbp_player))
    (set `self.CurrentSocket` (`SpringArmComponent.SocketOffset` _springarm))
    (set `self.CurrentTarget` (`SpringArmComponent.TargetOffset` _springarm))
    (set `self.CurrentLength` (`SpringArmComponent.TargetArmLength` _springarm))
    (set `self.CurrentRotation` (`SceneComponent.K2_GetComponentRotation` (`/Game/Blueprints/Players/BP_Player.FollowCamera` _asbp_player)))
    (bind _returnvalue_2 (`KismetSystemLibrary.K2_SetTimerDelegate` (delegate `setSpring`) 0.005 true))))

(event `setSpring`
  (bind _alpha (`self.alpha`))
  (bind _characterref (`self.characterRef`))
  (bind _springarm (`/Game/Blueprints/Players/BP_Player.SpringArm` _characterref))
  (set `SpringArmComponent.TargetOffset` (`KismetMathLibrary.VLerp` (`self.CurrentTarget`) (`self.Target Offset`) _alpha) _springarm)
  (set `SpringArmComponent.SocketOffset` (`KismetMathLibrary.VLerp` (`self.CurrentSocket`) (`self.Socket Offset`) _alpha) _springarm)
  (set `SpringArmComponent.TargetArmLength` (`KismetMathLibrary.Lerp` (`self.CurrentLength`) (`self.Arm Length`) _alpha) _springarm)
  (`SceneComponent.K2_SetWorldRotation` (`/Game/Blueprints/Players/BP_Player.FollowCamera` _characterref) (`KismetMathLibrary.RLerp` (`self.CurrentRotation`) (`self.CameraRotation`) (`self.alpha`)) false false)
  (set `self.alpha` (+ (`self.alpha`) 0.005))
  (if (== (`self.alpha`) 1.0)
    (`KismetSystemLibrary.K2_ClearAndInvalidateTimerHandle` (stale `self.Box.OnComponentBeginOverlap` _returnvalue_2))
    (set `self.alpha` 0.1)))

(fn `Set Spring Arm`
  (bind _springarm (`/Game/Blueprints/Players/BP_Player.SpringArm` (`self.characterRef`)))
  (set `SpringArmComponent.TargetOffset` (`self.Target Offset`) _springarm)
  (set `SpringArmComponent.SocketOffset` (`self.Socket Offset`) _springarm)
  (set `SpringArmComponent.TargetArmLength` (`self.Arm Length`) _springarm))

(fn `UserConstructionScript`
  (bind _springarm (`/Game/Blueprints/Players/BP_Player.SpringArm` (`self.characterRef`)))
  (set `SpringArmComponent.TargetOffset` (`self.Target Offset`) _springarm)
  (set `SpringArmComponent.SocketOffset` (`self.Socket Offset`) _springarm)
  (set `SpringArmComponent.TargetArmLength` (`self.Arm Length`) _springarm))
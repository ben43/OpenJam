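; BP_FadingWalls is a utility Blueprint that fades its static mesh out or back in through a material parameter.
; BeginPlay creates a dynamic instance of the mesh's first material.
; Each FadeMaterial call alternates between playing and reversing the Alpha timeline, which drives the material's Alpha scalar.
; A DoOnce gate blocks further calls until the timeline finishes and ResetTimeline reopens it.
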(event `self.ReceiveBeginPlay`
  (bind _staticmeshcomponent (`self.StaticMeshComponent`))
  (bind _returnvalue (`PrimitiveComponent.CreateDynamicMaterialInstance` _staticmeshcomponent 0 (`PrimitiveComponent.GetMaterial` _staticmeshcomponent 0) "None"))
  (set `self.MaterialRef` _returnvalue))

(event `/Game/Blueprints/BPi_Interact.FadeMaterial`
  (`/Engine/EditorBlueprintResources/StandardMacros.DoOnce` false :!label _label
    (:`Completed`
      (`/Engine/EditorBlueprintResources/StandardMacros.FlipFlop`
        (:`A`
          (bind (_direction _newtrack_0) (`Timeline|Alpha` :!via `PlayFromStart` :!label _label_2)
            (:`Update`
              (`MaterialInstanceDynamic.SetScalarParameterValue` (`self.MaterialRef`) "Alpha" _newtrack_0))
            (:`Finished`
              (`self.ResetTimeline`))))
        (:`B`
          (goto _label_2 :!via `ReverseFromEnd`))))))

(event `ResetTimeline`
  (goto _label :!via `Reset`))

(fn `UserConstructionScript`)
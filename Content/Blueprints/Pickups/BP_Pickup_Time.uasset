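; BP_Pickup_Time is a time bonus pickup, a child Blueprint that supplies the pickup action.
; The action adds AddedTime to the Time value on myGameState and shows the added amount through the player's HUD reference.
; It then destroys itself and plays a 2D pickup sound once, guarded by a DoOnce.
; Its event graph holds only disabled default events, and the construction script just calls the parent.
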(fn `Pickup_action`
  (bind _addedtime (`self.AddedTime`))
  (bind _asmy_game_state (cast `/Game/Blueprints/myGameState` (`GameplayStatics.GetGameState`)))
  (set `/Game/Blueprints/myGameState.Time` (+ (`/Game/Blueprints/myGameState.Time` _asmy_game_state) _addedtime) _asmy_game_state)
  (message `/Game/Blueprints/BPi_Interact.HudAddTime` (`/Game/Blueprints/Players/BP_Player.PlayerHUDRef` (`self.PlayerRef`)) _addedtime)
  (`self.K2_DestroyActor`)
  (`/Engine/EditorBlueprintResources/StandardMacros.DoOnce` false
    (:`Completed`
      (`GameplayStatics.SpawnSound2D` "/Game/Audio/Cues/A_Cue_PickupTime.A_Cue_PickupTime" 1.0 1.0 0.0 null))))

(fn `UserConstructionScript`
  (`parent.UserConstructionScript`))
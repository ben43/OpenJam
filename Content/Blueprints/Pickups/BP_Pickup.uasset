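; BP_Pickup is a pickup actor that the player collects by touching it.
; On BeginPlay it caches references to the player and the chaser, though its own graphs never use them.
; When the box hitbox overlaps player character 0, it prints the item name, hides its mesh and calls PickupAction, which only destroys the actor.
; Overlaps from other actors just print a debug "false".
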(event `self.ReceiveBeginPlay`
  (`|ExecutionSequence`
    (:`then_0`
      (bind _returnvalue (`/Game/Blueprints/FunctionLibrary.GetPlayerReference`))
      (set `self.PlayerRef` _returnvalue))
    (:`then_1`
      (bind _returnvalue_2 (`/Game/Blueprints/FunctionLibrary.GetChaserReference`))
      (set `self.ChaserRef` _returnvalue_2))))

(event `self.hitbox_Boxcolide.OnComponentBeginOverlap`
  (params (OverlappedComponent :type "PrimitiveComponent Object Reference") (OtherActor :type "Actor Object Reference") (OtherComp :type "PrimitiveComponent Object Reference") (OtherBodyIndex :type Integer) (bFromSweep :type Boolean) (SweepResult :type "HitResult Structure (by ref)"))
  ;[1 1 1] detect overlap and call function
  (if (== OtherActor (`GameplayStatics.GetPlayerCharacter` 0))
    (`KismetSystemLibrary.PrintString` (`self.itempickup_name`))
    (`SceneComponent.SetVisibility` (`self.Texture_mesh`) false false)
    (`self.Pickup_action`)
    (else
      (`KismetSystemLibrary.PrintString` "false"))))

(fn `Pickup_action`
  (`self.K2_DestroyActor`))

(fn `UserConstructionScript`)
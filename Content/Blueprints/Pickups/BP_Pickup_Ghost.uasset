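; Ghost pickup that lets pawns pass through an object in line with the player, as a child of a pickup base that handles overlap.
; PickupAction line-traces from player character 0 along its mesh's forward vector, with persistent debug drawing and a debug print.
; It sets the hit component's Pawn collision response to Overlap, with no hit check or revert, then destroys the pickup.
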(event `self.ReceiveActorBeginOverlap`
  (params (OtherActor :type "Actor Object Reference"))
  (`parent.ReceiveActorBeginOverlap` OtherActor))

(fn `Pickup_action`
  (locals (ObjectTypes :type "Array of EObjectTypeQuery Enum"))
  (bind _returnvalue (`GameplayStatics.GetPlayerCharacter` 0))
  (bind _returnvalue_2 (`self.K2_GetActorLocation` _returnvalue))
  (`KismetSystemLibrary.PrintString` "GHOSTING")
  (bind _outhit (`KismetSystemLibrary.LineTraceSingleForObjects` :`Start` _returnvalue_2 :`End` (+ _returnvalue_2 (* (`KismetMathLibrary.GetForwardVector` (`SceneComponent.K2_GetComponentRotation` (`Character.Mesh` _returnvalue))) 1000.0)) :`ObjectTypes` (`local.ObjectTypes`) :`DrawDebugType` "Persistent"))
  (`PrimitiveComponent.SetCollisionResponseToChannel` (`.HitComponent` (`GameplayStatics.BreakHitResult` _outhit)) "ECC_Pawn" "ECR_Overlap")
  (`self.K2_DestroyActor`))

(fn `UserConstructionScript`
  (`parent.UserConstructionScript`))
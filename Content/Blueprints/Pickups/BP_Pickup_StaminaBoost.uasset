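; Stamina boost pickup that raises the player's stamina when its pickup action runs.
; It overrides PickupAction to print a green on-screen message, add StaminaBoost to PlayerRef's Stamina with no clamp in this graph, then destroy itself.
; The event graph holds only disabled default events, and nothing here sets PlayerRef or calls PickupAction.
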(fn `Pickup_action`
  (locals (Max_speed :type "Float (double-precision)" :default 1500.0))
  (bind _playerref (`self.PlayerRef`))
  (`KismetSystemLibrary.PrintString` "Stamina Boost!" true true (struct :`R` 0.035066 :`G` 1.0 :`B` 0.269266 :`A` 1.0))
  (set `/Game/Blueprints/Players/BP_Player.Stamina` (+ (`/Game/Blueprints/Players/BP_Player.Stamina` _playerref) (`self.StaminaBoost`)) _playerref)
  (`self.K2_DestroyActor`))

(fn `UserConstructionScript`
  (`parent.UserConstructionScript`))
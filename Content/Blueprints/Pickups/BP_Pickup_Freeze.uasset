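; Freeze pickup that temporarily stops the Chaser character from moving.
; PickupAction destroys the hitbox and light, disables the Chaser's CharacterMovement, and plays a blue-tinted particle burst with a one-shot sound.
; A timer set by function name runs for FreezeTime; ReEnableMovement restores walking and destroys the pickup.
; Freeze and unfreeze print debug strings, and the event graph holds only disabled default nodes.
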(fn `Disable_movement`
  (`KismetSystemLibrary.PrintString` "Chaser Freezed!" true true (struct :`R` 1.0 :`G` 0.227157 :`B` 0.197308 :`A` 1.0))
  (`ActorComponent.K2_DestroyComponent` (`self.PointLight`))
  (`CharacterMovementComponent.DisableMovement` (`Character.CharacterMovement` (`self.ChaserRef`)))
  (bind _returnvalue (`NiagaraFunctionLibrary.SpawnSystemAtLocation` "/Game/FX/PS_Pickup.PS_Pickup" (`self.K2_GetActorLocation`)))
  (`FXSystemComponent.SetColorParameter` _returnvalue "Color" (struct :`R` 0.120794 :`G` 0.467687 :`B` 1.0 :`A` 1.0)))

(fn `Pickup_action`
  (locals (Freeze_time :type "Float (double-precision)" :default 3.0))
  (`ActorComponent.K2_DestroyComponent` (`self.hitbox_Boxcolide`))
  (`self.Disable_movement`)
  (`KismetSystemLibrary.K2_SetTimer` null (`self.functionToCall`) (`local.Freeze_time`))
  (`/Engine/EditorBlueprintResources/StandardMacros.DoOnce` false
    (:`Completed`
      (`GameplayStatics.SpawnSound2D` "/Game/Audio/Cues/A_Cue_PickupFreeze.A_Cue_PickupFreeze" 2.0 1.0 0.0 null))))

(fn `ReEnable_movement`
  (`KismetSystemLibrary.PrintString` "Chaser unfroze" true true (struct :`R` 0.151403 :`G` 1.0 :`B` 0.13291 :`A` 1.0))
  (`CharacterMovementComponent.SetMovementMode` (`Character.CharacterMovement` (`self.ChaserRef`)) "MOVE_Walking" 0)
  (`self.K2_DestroyActor`))

(fn `UserConstructionScript`
  (`parent.UserConstructionScript`))